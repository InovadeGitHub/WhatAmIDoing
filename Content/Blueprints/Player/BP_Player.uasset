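; Player actor that leans toward the mouse cursor and spawns an actor into the scene on left click.
; Each tick it remaps look-at pitch and yaw to the deprojected cursor into narrow clamped ranges and smoothly interpolates its rotation.
; A click calls the Linetrace helper along the cursor ray and spawns at the trace's end point, not the impact, with a pop sound.
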(event `self.ReceiveTick`
  (params (DeltaSeconds :type "Float (single-precision)"))
  (bind _returnvalue_roll (`KismetMathLibrary.BreakRotator` (`self.K2_GetActorRotation`)))
  (bind (_returnvalue_roll_2 _returnvalue_pitch _returnvalue_yaw) (`KismetMathLibrary.BreakRotator` (`KismetMathLibrary.FindLookAtRotation` (`self.K2_GetActorLocation`) (`PlayerController.DeprojectMousePositionToWorld` (`GameplayStatics.GetPlayerController` 0)))))
  ;[0.6 0.01 0] Tick
  (`self.K2_SetActorRotation` (`KismetMathLibrary.RInterpTo` (`self.K2_GetActorRotation`) (`KismetMathLibrary.MakeRotator` _returnvalue_roll (`KismetMathLibrary.MapRangeClamped` _returnvalue_pitch 38.0 -38.0 5.0 -5.0) (`KismetMathLibrary.MapRangeClamped` _returnvalue_yaw 125.0 -125.0 15.0 -15.0)) (`GameplayStatics.GetWorldDeltaSeconds`) 2.0)))

(event `Key|LeftMouseButton`
  (params (Key :type "Key Structure"))
  ;[0.4 1 0.1] Spawn Object
  (:`Pressed`
    (bind _outhit (`self.Linetrace` 1250.0))
    (`|SpawnActorFromClass` "/Game/Blueprints/Objects/BP_BaseSpawnable.BP_BaseSpawnable_C" (`KismetMathLibrary.MakeTransform` (`.TraceEnd` (`GameplayStatics.BreakHitResult` _outhit))) "Undefined" "OverrideRootScale" null null)
    (`GameplayStatics.PlaySound2D` "/Game/Audio/SoundEffects/Pop/CUE_Pop.CUE_Pop" 1.0 1.0 0.0 null null)))

(fn `Linetrace`
  (params (TraceLength :type "Float (double-precision)" :default 1000.0) (DrawDebug :type Boolean))
  (returns (OutHit :type "HitResult Structure") (ReturnValue :type Boolean))
  (bind (_worldlocation _worlddirection) (`PlayerController.DeprojectMousePositionToWorld` (`GameplayStatics.GetPlayerController` 0)))
  (bind (_outhit _returnvalue) (`KismetSystemLibrary.LineTraceSingle` :`Start` _worldlocation :`End` (+ _worldlocation (* _worlddirection (`local.TraceLength`))) :`TraceChannel` "TraceTypeQuery1" :`DrawDebugType` (select `bool` (`local.DrawDebug`) :!type "EDrawDebugTrace Enum")))
  (return _outhit _returnvalue))

(fn `UserConstructionScript`)