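; Single-use launch pad that throws the first overlapping BP_BaseSpawnable upward.
; A box overlap passes through a DoOnce with no reset, then applies a random vertical velocity-change impulse to the spawnable's mesh.
; The pad starts green and turns red on firing, recoloring the launched object pink-red as well.
; SetAppearance drives both a dynamic material's color parameter and the point light.
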(event `self.ReceiveBeginPlay`
  (bind _returnvalue (`PrimitiveComponent.CreateDynamicMaterialInstance` (`self.StaticMesh`) 0 null "None"))
  (set `self.Spawnable Material` _returnvalue))

(event `self.Box.OnComponentBeginOverlap`
  (params (OverlappedComponent :type "PrimitiveComponent Object Reference") (OtherActor :type "Actor Object Reference") (OtherComp :type "PrimitiveComponent Object Reference") (OtherBodyIndex :type Integer) (bFromSweep :type Boolean) (SweepResult :type "HitResult Structure (by ref)"))
  (bind _asbp_base_spawnable (cast `/Game/Blueprints/Objects/BP_BaseSpawnable` OtherActor))
  (`/Engine/EditorBlueprintResources/StandardMacros.DoOnce` false
    (:`Completed`
      (`PrimitiveComponent.AddImpulse` (`/Game/Blueprints/Objects/BP_BaseSpawnable.StaticMesh` _asbp_base_spawnable) (`KismetMathLibrary.MakeVector` 0.0 0.0 (`KismetMathLibrary.RandomFloatInRange` 1600.0 2200.0)) "None" true)
      (`self.Set Appearance` (struct :`R` 1.0 :`A` 1.0))
      (`/Game/Blueprints/Objects/BP_BaseSpawnable.Set Appearance` _asbp_base_spawnable (struct :`R` 1.0 :`B` 0.5 :`A` 1.0)))))

(fn `Set Appearance`
  (params (SpawnableColor :type "LinearColor Structure" :default (struct :`R` 0.4 :`G` 1.0 :`A` 1.0)))
  (`MaterialInstanceDynamic.SetVectorParameterValue` (`self.Spawnable Material`) "Color" SpawnableColor)
  (`LightComponent.SetLightColor` (`self.PointLight`) SpawnableColor true))

(fn `UserConstructionScript`
  (bind _returnvalue (`PrimitiveComponent.CreateDynamicMaterialInstance` (`self.StaticMesh`) 0 null "None"))
  (set `self.Spawnable Material` _returnvalue)
  (`MaterialInstanceDynamic.SetVectorParameterValue` (`self.Spawnable Material`) "Color" (struct :`R` 0.4 :`G` 1.0 :`A` 1.0))
  (`LightComponent.SetLightColor` (`self.PointLight`) (struct :`R` 0.4 :`G` 1.0 :`A` 1.0) true))