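; BP_BaseSpawnable is a base spawnable object with a colored mesh and matching point light.
; Construction applies SpawnableColor through a dynamic material; BeginPlay creates and caches another for SetAppearance.
; A hit while the actor moves fast enough calls SetAppearance to turn material and light red.
; BeginPlay also rolls a random per-axis scale for a TL_Spawn grow-from-zero timeline, which nothing in this graph starts.
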(event `self.ReceiveBeginPlay`
  (bind _returnvalue (`KismetMathLibrary.RandomFloatInRange` 1.0 1.25))
  (bind _returnvalue_2 (`PrimitiveComponent.CreateDynamicMaterialInstance` (`self.StaticMesh`) 0 null "None"))
  (set `self.Spawnable Material` _returnvalue_2)
  (set `self.Randomized Scale` (`KismetMathLibrary.MakeVector` _returnvalue _returnvalue _returnvalue)))

(event `self.StaticMesh.OnComponentHit`
  (params (HitComponent :type "PrimitiveComponent Object Reference") (OtherActor :type "Actor Object Reference") (OtherComp :type "PrimitiveComponent Object Reference") (NormalImpulse :type "Vector Structure") (Hit :type "HitResult Structure (by ref)"))
  (if (>= (`KismetMathLibrary.VSize` (`self.GetVelocity`)) 100.0)
    (`self.Set Appearance` (struct :`R` 1.0 :`A` 1.0))))

(fn `Set Appearance`
  (params (SpawnableColor :type "LinearColor Structure" :default (struct :`R` 0.05 :`G` 0.5 :`B` 1.0 :`A` 1.0)))
  (`MaterialInstanceDynamic.SetVectorParameterValue` (`self.Spawnable Material`) "Color" SpawnableColor)
  (`LightComponent.SetLightColor` (`self.PointLight`) SpawnableColor true))

(fn `UserConstructionScript`
  (bind _spawnable_color (`self.Spawnable Color`))
  (bind _returnvalue (`PrimitiveComponent.CreateDynamicMaterialInstance` (`self.StaticMesh`) 0 null "None"))
  (`MaterialInstanceDynamic.SetVectorParameterValue` _returnvalue "Color" _spawnable_color)
  (`LightComponent.SetLightColor` (`self.PointLight`) _spawnable_color true))